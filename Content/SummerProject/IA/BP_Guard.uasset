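; BP_Guard is a guard AI that runs the BT_Guard behavior tree and feeds it objective positions from its Routine.
; On BeginPlay it starts the tree on its AI controller and writes the Routine's current objective position to the InteractablePosition blackboard key.
; Each Routine index change rewrites that key and prints the new index, so the Blueprint only bridges the Routine to the blackboard.
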(event OnIndexChanged(Routine)
  (params (newIndex :type Integer))
  (AI|Components|Blackboard|SetValueasVector (AI|GetBlackboard (AI|GetAIController self)) (Utilities|Name|MakeLiteralName "InteractablePosition") (Class|RoutineComponent|GetCurrentObjectivePosition (Variables|Default|GetRoutine)))
  (Development|PrintString (Utilities|String|ToString(Integer) newIndex)))

(event EventBeginPlay
  (bind _self self)
  (bind _returnvalue (AI|GetAIController _self))
  (AI|RunBehaviorTree _returnvalue "/Game/SummerProject/IA/BT_Guard.BT_Guard")
  (AI|Components|Blackboard|SetValueasVector (AI|GetBlackboard _returnvalue) (Utilities|Name|MakeLiteralName "InteractablePosition") (Class|RoutineComponent|GetCurrentObjectivePosition (Variables|Default|GetRoutine))))

(fn ConstructionScript)